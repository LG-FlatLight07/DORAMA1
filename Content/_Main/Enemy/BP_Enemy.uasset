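; BP_Enemy is a rifle-armed AI enemy that wanders, turns toward the player and fires on sighting them.
; Perception of BP_Character sets IsSee, waits, adds ammo, then loops montages, muzzle flash and sound until ammo or HP runs out.
; Tick handles the death montage, smooth rotation toward the player while IsSee, and delayed random-point AIMoveTo otherwise.
; Firing is cosmetic here, with no trace, projectile or damage.
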(event OnTargetPerceptionUpdated(AIPerception)
  (params (Actor :type Actor%20Object%20Reference) (Stimulus :type AI%20Stimulus%20Structure))
  (Utilities|Casting|CastToBP_Character Actor)
  (if (not (Variables|Default|GetIsSee))
    (Variables|Default|SetIsSee true)
    (Utilities|FlowControl|Delay 5.0)
    (Variables|Default|SetCurrentAmmo (+ (Variables|Default|GetCurrentAmmo) (Variables|Default|GetMaxAmmo)))
    (if (not (<= (Variables|Default|GetHP) 0.0))
      ;[1 1 1] 射撃処理
      (Animation|Montage|PlayMontage (Variables|Character|GetMesh) "/Game/_Main/Animation/Fire_Rifle_Ironsights_Montage.Fire_Rifle_Ironsights_Montage" :!label _label
        (:then
          (Animation|Montage|PlayMontage (Variables|Default|GetAK) "/Game/_Main/Animation/Fire_Rifle_Ironsights_Montage.Fire_Rifle_Ironsights_Montage"
            (:then
              (Effects|SpawnEmitterAttached "/Game/MilitaryWeapDark/FX/P_AssaultRifle_MuzzleFlash.P_AssaultRifle_MuzzleFlash" (Variables|Default|GetAK) "Muzzle" "0.000000, 0, 0" "0, 0, 0" "1.000000,1.000000,1.000000" "SnapToTargetIncludingScale")
              (Audio|PlaySoundatLocation "/Game/MilitaryWeapDark/Sound/Rifle/RifleB_Fire_Cue.RifleB_Fire_Cue" (Transformation|GetSocketLocation (Variables|Character|GetMesh) "None") "0, 0, 0" 1.0 1.0 0.0 0 0 0)
              (Development|PrintString (Utilities|String|ToString(Byte) (Math|Conversions|ToByte(Integer) (Variables|Default|GetCurrentAmmo))))
              (if (<= (Variables|Default|GetCurrentAmmo) 0)
                (Variables|Default|SetIsSee false)
                (else
                  (Variables|Default|SetCurrentAmmo (- (Variables|Default|GetCurrentAmmo) 1))
                  (Utilities|FlowControl|Delay 0.1)
                  (if (not (<= (Variables|Default|GetHP) 0.0))
                    (goto _label)))))))))))

(event Custom|PlayMontage
  (Animation|Montage|PlayMontage (Variables|Character|GetMesh) "/Game/_Main/Animation/Fire_Rifle_Ironsights_Montage.Fire_Rifle_Ironsights_Montage"))

(event Custom|Attack
  (Animation|Montage|PlayMontage (Variables|Character|GetMesh) "/Game/_Main/Animation/Fire_Rifle_Ironsights_Montage.Fire_Rifle_Ironsights_Montage"))

(event EventTick
  (params (DeltaSeconds :type Float%20%28single-precision%29))
  ;[1 1 1] 志望理由処理
  (if (<= (Variables|Default|GetHP) 0.0)
    (if (not (Variables|Default|GetIsDead))
      (Variables|Default|SetIsDead true)
      (Animation|Montage|PlayMontage (Variables|Character|GetMesh) "/Game/_Main/Enemy/Death_1_Montage.Death_1_Montage"))
    (else
      ;[1 1 1] 角度変更
      (if (Variables|Default|GetIsSee)
        (Transformation|SetActorRotation (Math|Interpolation|RInterpTo (Transformation|GetActorRotation) (Math|Rotator|FindLookatRotation (Transformation|GetActorLocation) (Transformation|GetActorLocation (Variables|Default|GetPlayer))) (Utilities|Time|GetWorldDeltaSeconds) 2.0))
        (else
          (Utilities|FlowControl|Delay (Math|Random|RandomFloatinRange 1.0 3.0))
          (Variables|Default|SetIsMoving true)
          (AI|AIMoveTo self (.RandomLocation (AI|Navigation|GetRandomReachablePointinRadius (Transformation|GetActorLocation) 1.5e+03 0 0)) 0 5.0 false
            (:OnSuccess
              _)
            (:OnFail
              _))
          (Variables|Default|SetIsMoving false))))))

(event EventBeginPlay
  (bind _returnvalue (Actor|GetActorOfClass "/Game/_Main/Character/BP_Character.BP_Character_C"))
  (Variables|Default|SetPlayer _returnvalue))

(fn ConstructionScript)

(fn DeadCheck
  (if (<= (Variables|Default|GetHP) 0.0)
    (Components|Animation|PlayAnimation (Variables|Character|GetMesh) "/Game/_Main/Enemy/Death_1_Montage.Death_1_Montage" false)
    (Development|PrintString "Hello")))